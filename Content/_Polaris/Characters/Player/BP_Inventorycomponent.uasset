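; Player inventory component that holds a ten-slot item array and shows it in a WB_Inventory widget toggled with I.
; E runs a zero-length, debug-drawn sphere trace near the player's feet and casts the hit actor to read its Item.
; A slot loop stacks matching stackable items up to a limit or fills empty slots, then reloads the widget and destroys the actor.
; The loop has no break, so it continues after a slot is written.
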(event EventBeginPlay
  (bind _returnvalue (UserInterface|CreateWidget "/Game/Inventory/UI/WB_Inventory.WB_Inventory_C" 0 0))
  (Variables|Default|SetInventorywidget _returnvalue)
  (Utilities|Array|Resize (Variables|Default|GetItems) 10)
  (Default|LoadInventory (Variables|Default|GetInventorywidget) self))

(event EventTick
  (params (DeltaSeconds :type Float%20%28single-precision%29)))

(event Input|KeyboardEvents|I
  (params (Key :type Key%20Structure))
  (bind _inventorywidget (Variables|Default|GetInventorywidget))
  (:Pressed
    (if (Widget|IsVisible (Variables|Default|GetInventorywidget))
      (Widget|RemovefromParent _inventorywidget)
      (else
        (UserInterface|Viewport|AddtoViewport _inventorywidget 0)))))

(event Input|KeyboardEvents|E
  (params (Key :type Key%20Structure))
  (bind _returnvalue (Game|GetPlayerCharacter 0))
  (bind _returnvalue_2 (Transformation|GetActorLocation _returnvalue))
  (bind _returnvalue_3 (- _returnvalue_2 "0.000000,0.000000,65.000000"))
  (:Pressed
    (bind _outhit (Collision|SphereTraceByChannel _returnvalue_3 _returnvalue_3 1.2e+02 "TraceTypeQuery1" false 0 "ForDuration"))
    (bind _asbp_item (Utilities|Casting|CastTo (.HitActor (Collision|BreakHitResult _outhit))))
    (for (_array_element _array_index) (Variables|Default|GetItems)
      (if (Math|Boolean|ANDBoolean (Utilities|Enum|Equal(Enum) (.Name (Utilities|Struct|BreakFallbackStruct _array_element)) (.Name (Utilities|Struct|BreakFallbackStruct (Variables|Default|GetItem _asbp_item)))) (.Stackable (Utilities|Struct|BreakFallbackStruct (Variables|Default|GetItem _asbp_item))) (<= (+ (.Quantity (Utilities|Struct|BreakFallbackStruct _array_element)) (.Quantity (Utilities|Struct|BreakFallbackStruct (Variables|Default|GetItem _asbp_item)))) 64))
        (Utilities|Array|SetArrayElem (Variables|Default|GetItems) _array_index (Utilities|Struct|MakeFallbackStruct (.name (Variables|Default|GetItem _asbp_item)) (.stackable (Variables|Default|GetItem _asbp_item)) (+ (.Quantity (Utilities|Struct|BreakFallbackStruct _array_element)) (.Quantity (Utilities|Struct|BreakFallbackStruct (Variables|Default|GetItem _asbp_item)))) (.thumnail (Variables|Default|GetItem _asbp_item)) (.mesh (Variables|Default|GetItem _asbp_item))))
        (Default|LoadInventory (Variables|Default|GetInventorywidget) self :!label _label)
        (Actor|DestroyActor _asbp_item)
        (elif (== (.Quantity (Utilities|Struct|BreakFallbackStruct _array_element)) 0)
          (Utilities|Array|SetArrayElem (Variables|Default|GetItems) _array_index (Variables|Default|GetItem _asbp_item))
          (goto _label))))))